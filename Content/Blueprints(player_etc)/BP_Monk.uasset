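; BP_Monk is a monk NPC Blueprint that shows a WBP_MonkNPC widget on screen while a BP_CCharacter is within range.
; Its Sphere's begin-overlap event creates the widget for player 0 on first use, caches it in UserWidget and adds it to the viewport.
; End overlap removes the widget from its parent, and later overlaps re-add the cached instance while it remains valid.
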(event OnComponentBeginOverlap(Sphere)
  (params (OverlappedComponent :type Primitive%20Component%20Object%20Reference) (OtherActor :type Actor%20Object%20Reference) (OtherComp :type Primitive%20Component%20Object%20Reference) (OtherBodyIndex :type Integer) (bFromSweep :type Boolean) (SweepResult :type Hit%20Result%20Structure%20%28by%20ref%29))
  (Utilities|Casting|CastToBP_CCharacter OtherActor)
  (Utilities|IsValid (Variables|Default|GetUserWidget)
    (:Is%20Valid
      (UserInterface|Viewport|AddtoViewport (Variables|Default|GetUserWidget) 0))
    (:Is%20Not%20Valid
      (bind _returnvalue (UserInterface|CreateWidget "/Game/HUD/WBP_MonkNPC.WBP_MonkNPC_C" (Game|GetPlayerController 0)))
      (Variables|Default|SetUserWidget _returnvalue)
      (UserInterface|Viewport|AddtoViewport _returnvalue 0))))

(event OnComponentEndOverlap(Sphere)
  (params (OverlappedComponent :type Primitive%20Component%20Object%20Reference) (OtherActor :type Actor%20Object%20Reference) (OtherComp :type Primitive%20Component%20Object%20Reference) (OtherBodyIndex :type Integer))
  (Utilities|Casting|CastToBP_CCharacter OtherActor)
  (Widget|RemovefromParent (Variables|Default|GetUserWidget)))

(event EventBeginPlay)

(event Collision|EventActorBeginOverlap
  (params (OtherActor :type Actor%20Object%20Reference)))

(event EventTick
  (params (DeltaSeconds :type Float%20%28single-precision%29)))

(fn ConstructionScript)