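; BP_Door is a door with two static meshes that swing in yaw when the custom DoorOpen event fires.
; Each mesh has its own timeline, whose vector track Z value is combined with a captured world rotation.
; The second timeline starts inside the first's Update, so it restarts and recaptures its mesh rotation on every update of the first.
; The box overlap event is empty, so DoorOpen relies on an external caller.
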(event OnComponentBeginOverlap(Box)
  (params (OverlappedComponent :type Primitive%20Component%20Object%20Reference) (OtherActor :type Actor%20Object%20Reference) (OtherComp :type Primitive%20Component%20Object%20Reference) (OtherBodyIndex :type Integer) (bFromSweep :type Boolean) (SweepResult :type Hit%20Result%20Structure%20%28by%20ref%29)))

(event Custom|DoorOpen
  ;[1 1 1] 원하는 이벤트에 실행
  (Variables|Default|SetMesh1Rot (Transformation|GetWorldRotation (Variables|Default|GetStaticMesh1)))
  (bind _새_트랙_1 (Timeline|타임라인 PlayFromStart)
    (:Update
      (Transformation|SetWorldRotation (Variables|Default|GetStaticMesh1) (Math|Rotator|CombineRotators (Math|Rotator|MakeRotator 0.0 0.0 (.Z (Math|Vector|BreakVector _새_트랙_1))) (Variables|Default|GetMesh1Rot)) false false)
      (Variables|Default|SetMeshRot (Transformation|GetWorldRotation (Variables|Default|GetStaticMesh)))
      (bind _새_트랙_1_2 (Timeline|타임라인_0 PlayFromStart)
        (:Update
          (Transformation|SetWorldRotation (Variables|Default|GetStaticMesh) (Math|Rotator|CombineRotators (Math|Rotator|MakeRotator 0.0 0.0 (.Z (Math|Vector|BreakVector _새_트랙_1_2))) (Variables|Default|GetMeshRot)) false false))))))

(event EventBeginPlay)

(event Collision|EventActorBeginOverlap
  (params (OtherActor :type Actor%20Object%20Reference)))

(event EventTick
  (params (DeltaSeconds :type Float%20%28single-precision%29)))

(fn ConstructionScript)