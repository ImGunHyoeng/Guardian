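; BP_Antiquity is an antiquity (relic) actor that shows a detail window while the player character is near it.
; BeginPlay creates a WBP_DetailWindow and sets its image from the actor's Name.
; Box overlap with BP_CCharacter sets itself as that character's Antiquity and displays the window; leaving clears both.
; An inventory pickup chain that activates the item by Name and destroys the actor is present but never runs.
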(event OnComponentBeginOverlap(Box)
  (params (OverlappedComponent :type Primitive%20Component%20Object%20Reference) (OtherActor :type Actor%20Object%20Reference) (OtherComp :type Primitive%20Component%20Object%20Reference) (OtherBodyIndex :type Integer) (bFromSweep :type Boolean) (SweepResult :type Hit%20Result%20Structure%20%28by%20ref%29))
  ;[1 1 1] UI 띄우기
  (bind _asbp_ccharacter (Utilities|Casting|CastToBP_CCharacter OtherActor))
  (Variables|/Game/Blueprints(player_etc)/BP_CCharacter.BP_CCharacter_C|SetAntiquity _asbp_ccharacter self)
  (UserInterface|Viewport|AddtoViewport (Variables|Default|GetDetail) 0))

(event OnComponentEndOverlap(Box)
  (params (OverlappedComponent :type Primitive%20Component%20Object%20Reference) (OtherActor :type Actor%20Object%20Reference) (OtherComp :type Primitive%20Component%20Object%20Reference) (OtherBodyIndex :type Integer))
  ;[1 1 1] 초기화
  (bind _asbp_ccharacter (Utilities|Casting|CastToBP_CCharacter OtherActor))
  (Variables|/Game/Blueprints(player_etc)/BP_CCharacter.BP_CCharacter_C|SetAntiquity _asbp_ccharacter 0)
  (Widget|RemovefromParent (Variables|Default|GetDetail)))

(event EventBeginPlay
  ;[1 1 1] 유물 UI
  (bind _returnvalue (UserInterface|CreateWidget "/Game/HUD/WBP_DetailWindow.WBP_DetailWindow_C" (Game|GetPlayerController 0)))
  (Variables|Default|SetDetail _returnvalue)
  (Default|SetImageF (Variables|Default|GetDetail) (Variables|Default|GetName)))

(event Collision|EventActorBeginOverlap
  (params (OtherActor :type Actor%20Object%20Reference)))

(event EventTick
  (params (DeltaSeconds :type Float%20%28single-precision%29)))

(fn ConstructionScript)