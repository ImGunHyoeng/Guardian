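; Player character Blueprint that handles relic (Antiquity) pickup into the inventory and toggles the weapon's Niagara effect.
; BeginPlay caches the inventory widget, and a debug E key activates the item by the relic's name, then destroys the relic.
; GetHit only forwards to the parent.
; Damage and mesh collision events are empty, with disconnected leftovers for minimap, hit effects and ragdoll; a helper teleports the actor to its capsule's location.
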(event OnComponentHit(Mesh)
  (params (HitComponent :type Primitive%20Component%20Object%20Reference) (OtherActor :type Actor%20Object%20Reference) (OtherComp :type Primitive%20Component%20Object%20Reference) (NormalImpulse :type Vector :default "0, 0, 0") (Hit :type Hit%20Result%20Structure%20%28by%20ref%29)))

(event OnComponentBeginOverlap(Mesh)
  (params (OverlappedComponent :type Primitive%20Component%20Object%20Reference) (OtherActor :type Actor%20Object%20Reference) (OtherComp :type Primitive%20Component%20Object%20Reference) (OtherBodyIndex :type Integer) (bFromSweep :type Boolean) (SweepResult :type Hit%20Result%20Structure%20%28by%20ref%29)))

(event Custom|SetWarpTarget)

(event Custom|SetCapsuleLocation
  (Transformation|SetActorLocation (Transformation|GetWorldLocation (Variables|Default|GetCapsuleComponent)) false true))

(event EventBeginPlay
  ;[1 1 1] 인벤토리 위젯 변수 등록
  (bind _aswbp_inventory (Utilities|Casting|CastToWBP_Inventory (Variables|/Script/Caiman.InventoryComponent|GetItemWidget (Variables|Default|GetInventoryWidget))))
  (Variables|Default|SetAs%20WBP%20Inventory _aswbp_inventory))

(event Game|Damage|EventAnyDamage
  (params (Damage :type Float%20%28single-precision%29) (DamageType :type Damage%20Type%20Object%20Reference) (InstigatedBy :type Controller%20Object%20Reference) (DamageCauser :type Actor%20Object%20Reference))
  ;[1 1 1] 플레이어 피격처리
)

(event EventGetHit
  (params (ImpactPoint :type Vector%20%28by%20ref%29 :default "0, 0, 0") (Offense :type Actor%20Object%20Reference))
  (|CallParentFunction ImpactPoint Offense))

(event Game|Damage|EventPointDamage
  (params (Damage :type Float%20%28single-precision%29) (DamageType :type Damage%20Type%20Object%20Reference) (HitLocation :type Vector :default "0, 0, 0") (HitNormal :type Vector :default "0, 0, 0") (HitComponent :type Primitive%20Component%20Object%20Reference) (BoneName :type Name :default "None") (ShotFromDirection :type Vector :default "0, 0, 0") (InstigatedBy :type Controller%20Object%20Reference) (DamageCauser :type Actor%20Object%20Reference) (HitInfo :type Hit%20Result%20Structure%20%28by%20ref%29)))

(event EventDeActiveNaiagra
  (Components|Activation|SetActive (Variables|Default|GetNSWeapon) false true))

(event EventSetNaiagra
  (Components|Activation|SetActive (Variables|Default|GetNSWeapon) true false))

(event Input|KeyboardEvents|DebugKey1
  (params (Key :type Key%20Structure :default "None") (ActionValue :type Input%20Action%20Value%20Structure)))

(event Input|KeyboardEvents|DebugKeyE
  (params (Key :type Key%20Structure :default "None") (ActionValue :type Input%20Action%20Value%20Structure))
  (bind _antiquity (Variables|Default|GetAntiquity))
  ;[1 1 1] 유물 수집
  (:Pressed
    (Utilities|IsValid _antiquity
      (:Is%20Valid
        (Default|Active (Variables|Default|GetAs%20WBP%20Inventory) (Variables|/Game/Blueprints(player_etc)/BP_Antiquity.BP_Antiquity_C|GetName _antiquity))
        (Actor|DestroyActor _antiquity)))))

(fn ConstructionScript)