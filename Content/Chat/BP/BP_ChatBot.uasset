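; BP_ChatBot is an in-world chatbot actor that lets the player chat with an OpenAI model.
; Its sphere overlap creates or shows a WB_Chat widget when a BP_CCharacter enters and hides it on exit.
; ChatBotRequest appends input to a running ChatLog and sends the whole history asynchronously to GPT-4o, setting a currently blank API key.
; Successful replies join the log and go to the widget's Result; failures print the error.
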(event OnComponentBeginOverlap(Sphere)
  (params (OverlappedComponent :type Primitive%20Component%20Object%20Reference) (OtherActor :type Actor%20Object%20Reference) (OtherComp :type Primitive%20Component%20Object%20Reference) (OtherBodyIndex :type Integer) (bFromSweep :type Boolean) (SweepResult :type Hit%20Result%20Structure%20%28by%20ref%29))
  (Utilities|Casting|CastToBP_CCharacter OtherActor)
  (if (== (Variables|Default|GetAs%20WB%20Chat) 0)
    (bind _returnvalue (UserInterface|CreateWidget "/Game/Chat/HUD/WB_Chat.WB_Chat_C" (Game|GetPlayerController 0)))
    (UserInterface|Viewport|AddtoViewport _returnvalue 0)
    ;[1 1 1] 코멘트
    (if (== (Variables|Default|GetAs%20WB%20Chat) 0)
      (Variables|Default|SetAs%20WB%20Chat _returnvalue))
    (Widget|SetVisibility (Variables|Default|GetAs%20WB%20Chat) "Visible")
    (else
      (Widget|SetVisibility (Variables|Default|GetAs%20WB%20Chat) "Visible"))))

(event OnComponentEndOverlap(Sphere)
  (params (OverlappedComponent :type Primitive%20Component%20Object%20Reference) (OtherActor :type Actor%20Object%20Reference) (OtherComp :type Primitive%20Component%20Object%20Reference) (OtherBodyIndex :type Integer))
  (Utilities|Casting|CastToBP_CCharacter OtherActor)
  (if (not (== (Variables|Default|GetAs%20WB%20Chat) 0))
    (Widget|SetVisibility (Variables|Default|GetAs%20WB%20Chat) "Hidden")))

(event Custom|ChatBotRequest
  (params (input :type Chat%20Log%20Structure))
  (bind _chatlog (Variables|Default|GetChatLog))
  ;[1 1 1] API키 설정
  (Development|PrintString (.content (Utilities|Struct|BreakChatLog input)) false)
  (Class|OpenAIUtils|SetOpenAIApiKey)
  ;[1 1 1] null 체크
  (if (== (Variables|Default|GetAs%20WB%20Chat) 0)
    ;[1 1 1] 위젯 설정
    (bind _foundwidgets (Widget|GetAllWidgetsOfClass "/Game/Chat/HUD/WB_Chat.WB_Chat_C" true))
    (Variables|Default|SetAs%20WB%20Chat (Utilities|Array|Get(acopy) _foundwidgets)))
  ;[1 1 1] 지피티 4용 버전
  (Utilities|Array|Add _chatlog input)
  (bind (_message _errormessage _success) (|OpenAICallChat (Utilities|Struct|MakeChatSettings "GPT_4o_2024_08_06" _chatlog 0.2 400))
    (:Finished
      (if _success
        (Utilities|Array|Add (Variables|Default|GetChatLog) (.message (Utilities|Struct|BreakChatCompletion _message)))
        (Development|PrintString (.content (Utilities|Struct|BreakChatLog (.message (Utilities|Struct|BreakChatCompletion _message)))) false true "(R=0.000000,G=0.660000,B=1.000000,A=1.000000)" 1e+01)
        (Default|Result (Variables|Default|GetAs%20WB%20Chat) (Utilities|Text|ToText(String) (.content (Utilities|Struct|BreakChatLog (.message (Utilities|Struct|BreakChatCompletion _message))))))
        (else
          (Development|PrintString _errormessage false))))))

(event EventBeginPlay)

(event Collision|EventActorBeginOverlap
  (params (OtherActor :type Actor%20Object%20Reference)))

(event EventTick
  (params (DeltaSeconds :type Float%20%28single-precision%29)))

(fn ConstructionScript)