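; Enemy projectile that damages the player character (BP_CCharacter) and explodes on impact.
; Box overlap with the player applies damage, calls GetHit with the impact location, and also calls ApplyPointDamage.
; Player hits and overlaps with World Static components stop movement, hide the particles, play explosion sound and hit effect, then destroy the actor.
; A Delay on Tick destroys the projectile after a few seconds if nothing is hit.
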(event OnComponentHit(Box)
  (params (HitComponent :type Primitive%20Component%20Object%20Reference) (OtherActor :type Actor%20Object%20Reference) (OtherComp :type Primitive%20Component%20Object%20Reference) (NormalImpulse :type Vector :default "0, 0, 0") (Hit :type Hit%20Result%20Structure%20%28by%20ref%29))
  ;[1 1 1] 플레이어와 충돌처리
)

(event OnComponentBeginOverlap(Box)
  (params (OverlappedComponent :type Primitive%20Component%20Object%20Reference) (OtherActor :type Actor%20Object%20Reference) (OtherComp :type Primitive%20Component%20Object%20Reference) (OtherBodyIndex :type Integer) (bFromSweep :type Boolean) (SweepResult :type Hit%20Result%20Structure%20%28by%20ref%29))
  ;[1 1 1] 플레이어와 충돌처리
  (bind _asbp_ccharacter (Utilities|Casting|CastToBP_CCharacter OtherActor)
    (:then
      (Game|Damage|ApplyDamage _asbp_ccharacter (Variables|Default|GetBase%20Damage) 0 self "/Script/Engine.DamageType")
      (Class|HitInterface|GetHit _asbp_ccharacter (.location SweepResult) self)
      (Game|Damage|ApplyPointDamage 0 0.0 (.location SweepResult) (Collision|MakeHitResult false false 0.0 0.0 "0, 0, 0" "0, 0, 0" "0,0,1" "0,0,1" 0 0 0 (.hitbonename SweepResult) (.bonename SweepResult) 0 0 0 "0, 0, 0" "0, 0, 0") 0 self))
    (:CastFailed
      (switch Utilities|FlowControl|Switch|SwitchonECollisionChannel (Collision|GetCollisionObjectType OtherComp)
        (:ECC_WorldStatic
          _))))
  (Components|Movement|StopMovementImmediately (Variables|Default|GetProjectileMovement))
  (Rendering|SetVisibility (Variables|Default|GetParticleSystem) false false)
  (Audio|PlaySoundatLocation "/Game/Audio/Metasound/SFX_Explosion.SFX_Explosion" (Transformation|GetActorLocation) "0, 0, 0" 1.0 1.0 0.0 "/Game/Audio/MySoundAttenuation.MySoundAttenuation" 0 0 0)
  (Effects|SpawnEmitteratLocation "/Game/ParticleSystems/Fire_Bullet/Fire_Hit.Fire_Hit" (.location SweepResult) "0, 0, 0" "0.600000,0.600000,0.600000")
  (Actor|DestroyActor))

(event OnComponentWake(Box)
  (params (WakingComponent :type Primitive%20Component%20Object%20Reference) (BoneName :type Name :default "None"))
  ;[1 1 1] 플레이어와 충돌처리
)

(event EventBeginPlay)

(event Collision|EventActorBeginOverlap
  (params (OtherActor :type Actor%20Object%20Reference)))

(event EventTick
  (params (DeltaSeconds :type Float%20%28single-precision%29))
  (Utilities|FlowControl|Delay 6.0)
  (Actor|DestroyActor))

(fn ConstructionScript)