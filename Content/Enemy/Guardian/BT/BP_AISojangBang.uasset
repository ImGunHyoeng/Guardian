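; AI controller for the SojangBang Guardian enemy that runs BT_Solider on possess and seeds its Home and SelfActor blackboard keys.
; AI perception updates set HasLineOfSight and EnemyActor when an actor tagged Player is sensed, cancelling any pending forget timer.
; Any other perception update starts a delayed timer that clears both keys, so the enemy forgets its target after a grace period.
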(event OnTargetPerceptionUpdated(AIPerception)
  (params (Actor :type Actor%20Object%20Reference) (Stimulus :type AI%20Stimulus%20Structure))
  (bind _blackboard (Variables|Default|GetBlackboard))
  (if (Math|Boolean|ANDBoolean (.bSuccessfullySensed (Utilities|Struct|BreakAIStimulus Stimulus)) (Actor|ActorHasTag Actor "Player") true)
    ;[1 1 1] 플레이어일 경우 블랙보드의 키값 설정
    (Utilities|Time|ClearandInvalidateTimerbyHandle (stale _returnvalue))
    (Utilities|Time|ClearandInvalidateTimerbyHandle (Variables|Default|GetEnemy%20Timer))
    (AI|Components|Blackboard|SetValueasBool _blackboard (Variables|Default|GetHasLineOfSight) true)
    (AI|Components|Blackboard|SetValueasObject _blackboard (Variables|Default|GetEnemyActor) Actor)
    (else
      ;[1 1 1] AI가 인식한 것이 플레이어가 아닌 경우
      (bind _returnvalue (Utilities|Time|SetTimerbyEvent (delegate Custom|StartEnemyTimer) (Variables|Default|GetLine%20Of%20Sight%20Timer) false 6.0))
      (Variables|Default|SetEnemy%20Timer _returnvalue))))

(event Custom|StartEnemyTimer
  (bind _blackboard (Variables|Default|GetBlackboard))
  ;[1 1 1] AI가 인식한 것이 플레이어가 아닌 경우
  (AI|Components|Blackboard|SetValueasBool _blackboard (Variables|Default|GetHasLineOfSight) false)
  (AI|Components|Blackboard|SetValueasObject _blackboard (Variables|Default|GetEnemyActor) 0))

(event EventBeginPlay)

(event EventTick
  (params (DeltaSeconds :type Float%20%28single-precision%29)))

(event EventPossess
  (params (PossessedPawn :type Pawn%20Object%20Reference))
  ;[1 1 1] 행동트리 실행
  (AI|RunBehaviorTree "/Game/Enemy/Guardian/BT/BT_Solider.BT_Solider")
  (AI|Components|Blackboard|SetValueasVector (Variables|Default|GetBlackboard) (Variables|Default|GetHome) (Transformation|GetActorLocation (Components|GetOwner (Variables|Default|GetAIPerception))))
  (AI|Components|Blackboard|SetValueasObject (Variables|Default|GetBlackboard) (Variables|Default|GetSelfActor) self))

(fn ConstructionScript)