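; BP_SojangBang is a Guardian enemy Blueprint that handles melee attacks on the player and its own hit reactions.
; Overlap volumes track whether the player is in attack range and set widget visibility true on both entering and leaving detection.
; 공격판정 sphere-traces forward from the mesh, damages players through GetHit and ignores them until 공격끝남 clears the list.
; Incoming hits play a sword sound before calling the parent GetHit.
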(event OnComponentBeginOverlap(AttackStartRange)
  (params (OverlappedComponent :type Primitive%20Component%20Object%20Reference) (OtherActor :type Actor%20Object%20Reference) (OtherComp :type Primitive%20Component%20Object%20Reference) (OtherBodyIndex :type Integer) (bFromSweep :type Boolean) (SweepResult :type Hit%20Result%20Structure%20%28by%20ref%29))
  (Utilities|Casting|CastToBP_CCharacter OtherActor)
  (Variables|Default|SetAttackRange true))

(event OnComponentEndOverlap(AttackEndRange)
  (params (OverlappedComponent :type Primitive%20Component%20Object%20Reference) (OtherActor :type Actor%20Object%20Reference) (OtherComp :type Primitive%20Component%20Object%20Reference) (OtherBodyIndex :type Integer))
  (Utilities|Casting|CastToBP_CCharacter OtherActor)
  (Variables|Default|SetAttackRange false))

(event OnComponentBeginOverlap(DetectRange)
  (params (OverlappedComponent :type Primitive%20Component%20Object%20Reference) (OtherActor :type Actor%20Object%20Reference) (OtherComp :type Primitive%20Component%20Object%20Reference) (OtherBodyIndex :type Integer) (bFromSweep :type Boolean) (SweepResult :type Hit%20Result%20Structure%20%28by%20ref%29))
  (Utilities|Casting|CastToBP_CCharacter OtherActor)
  (Class|GuardianEnemyBase|SetWidgetVisible true))

(event OnComponentEndOverlap(DetectRange)
  (params (OverlappedComponent :type Primitive%20Component%20Object%20Reference) (OtherActor :type Actor%20Object%20Reference) (OtherComp :type Primitive%20Component%20Object%20Reference) (OtherBodyIndex :type Integer))
  (Utilities|Casting|CastToBP_CCharacter OtherActor)
  (Class|GuardianEnemyBase|SetWidgetVisible true))

(event Custom|공격판정
  (bind _mesh (Variables|Character|GetMesh))
  (bind _returnvalue (Transformation|GetSocketLocation _mesh "None"))
  (bind _outhits (Collision|MultiSphereTraceByChannel _returnvalue (+ _returnvalue (* (Math|Vector|GetForwardVector (Variables|Default|GetCapsuleComponent)) 300)) 5e+01 "TraceTypeQuery1" false (Variables|Default|GetActors%20to%20Ignore) "None"))
  (if (Utilities|Array|IsNotEmpty _outhits)
    (for _index (range 0 (Utilities|Array|Length _outhits))
      (bind _asccharacter_player (Utilities|Casting|CastToCCharacterPlayer (.HitActor (Collision|BreakHitResult (Utilities|Array|Get(acopy) _outhits _index)))))
      (Variables|Default|SetActors%20to%20Ignore (Utilities|Array|MakeArray _asccharacter_player))
      (Class|HitInterface|GetHit _asccharacter_player (.ImpactPoint (Collision|BreakHitResult (Utilities|Array|Get(acopy) _outhits _index))) self))))

(event Custom|공격%20끝남
  (Utilities|Array|Clear (Variables|Default|GetActors%20to%20Ignore)))

(event EventBeginPlay)

(event Collision|EventActorBeginOverlap
  (params (OtherActor :type Actor%20Object%20Reference)))

(event EventTick
  (params (DeltaSeconds :type Float%20%28single-precision%29)))

(event EventGetHit
  (params (ImpactPoint :type Vector%20%28by%20ref%29 :default "0, 0, 0") (Offense :type Actor%20Object%20Reference))
  (Audio|PlaySound2D "/Game/Audio/Metasound/SFX_SwordHit.SFX_SwordHit" 1.0 1.0 0.0 0 0)
  (|CallParentFunction ImpactPoint Offense))

(fn ConstructionScript)