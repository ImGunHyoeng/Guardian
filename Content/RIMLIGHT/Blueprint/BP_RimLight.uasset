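; BP_RimLight is an actor that animates a glow on the JunglimPagoda mesh.
; On BeginPlay it stores dynamic instances of the mesh's materials in Mat and starts a timeline.
; Each timeline update writes the truncated track value to Glow_Int on one instance, cycling CurNum through three slots.
; Despite the name, the rim light parameter logic is disconnected and never runs, and the construction script is empty.
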(event EventBeginPlay
  (bind _junglimpagoda (Variables|Default|GetJunglimPagoda))
  (for (_array_element _array_index) (Rendering|Material|GetMaterials _junglimpagoda)
    (bind _returnvalue (Rendering|Material|CreateDynamicMaterialInstance _junglimpagoda _array_index _array_element "None" :!class /Script/Engine.PrimitiveComponent))
    (Utilities|Array|SetArrayElem (Variables|Default|GetMat) _array_index _returnvalue)
    (bind _새_트랙_0 (Timeline|타임라인 Play)
      (:Update
        (Class|UMatetrialParameterHelper|SetIntParamifExists (Utilities|Array|Get(acopy) (Variables|Default|GetMat) (Variables|Default|GetCurNum)) "Glow_Int" (Math|Float|Truncate _새_트랙_0))
        (bind _result (Math|Integer|IncrementInt (Variables|Default|GetCurNum))
          (:%20%20
            (if (> _result 2)
              (Variables|Default|SetCurNum 0))))))))

(event Collision|EventActorBeginOverlap
  (params (OtherActor :type Actor%20Object%20Reference)))

(event EventTick
  (params (DeltaSeconds :type Float%20%28single-precision%29)))

(fn ConstructionScript)